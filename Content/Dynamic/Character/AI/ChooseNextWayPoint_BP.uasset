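; Behavior tree task for AI patrols, meant to pick the next waypoint from a list of patrol points.
; SetNextWayPoint writes the patrol point at the blackboard index to the WayPoints key, and Cycle advances that index, wrapping by array length.
; The execute event is unwired, so fetching points, both functions and FinishExecute never run, and the task does nothing and never finishes.
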(event `self.ReceiveExecuteAI`
  (params (OwnerController :type "AIController Object Reference") (ControlledPawn :type "Pawn Object Reference"))
  ;[1 1 1] c
)

(fn `Cycle`
  (bind _index (`self.Index`))
  (`BTFunctionLibrary.SetBlackboardValueAsInt` _index (mod (+ (`BTFunctionLibrary.GetBlackboardValueAsInt` _index) 1) (`KismetArrayLibrary.Array_Length` (`self.PatrolPoints`)))))

(fn `SetNextWayPoint`
  (`BTFunctionLibrary.SetBlackboardValueAsObject` (`self.WayPoints`) (`|GetArrayItem` (`self.PatrolPoints`) (`BTFunctionLibrary.GetBlackboardValueAsInt` (`self.Index`)))))