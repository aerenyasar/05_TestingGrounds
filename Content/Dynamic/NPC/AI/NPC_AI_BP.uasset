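; NPC AI controller that runs the guard behavior tree on patrol blackboard data.
; On BeginPlay it initializes the PatrolData blackboard, caches its component and starts GuardBehaviour.
; AI perception updates write sensed actors lacking the "Enemy" tag to the enemy key and clear that key when such an actor's stimulus is lost.
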(event `self.ReceiveBeginPlay`
  (bind _blackboardcomponent (`self.UseBlackboard` "/Game/Dynamic/NPC/AI/PatrolData.PatrolData"))
  (set `self.BBComp` _blackboardcomponent)
  (`self.RunBehaviorTree` "/Game/Dynamic/NPC/AI/GuardBehaviour.GuardBehaviour"))

(event `self.AIPerception.OnTargetPerceptionUpdated`
  (params (Actor :type "Actor Object Reference") (Stimulus :type "AIStimulus Structure"))
  (bind _bbcomp (`self.BBComp`))
  (bind _enemykey (`self.EnemyKey`))
  (if (`self.ActorHasTag` Actor "Enemy")
    _
    (elif (`.bSuccessfullySensed` (break `AIStimulus` Stimulus))
      (`BlackboardComponent.SetValueAsObject` _bbcomp _enemykey Actor)
      (else
        (`BlackboardComponent.ClearValue` _bbcomp _enemykey)))))

(fn `UserConstructionScript`)